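; Main menu game mode for a two-player Tron game where each player picks a power before the match.
; BeginPlay creates the UI_MainMenu widget, adds it to the viewport and shows the mouse cursor.
; Tick polls both players' ready checkboxes; once both are checked, it copies the selected powers into TronGameInstance and opens the Game level.
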(event `self.ReceiveBeginPlay`
  (bind _returnvalue (`GameplayStatics.GetPlayerController` 0))
  (bind _returnvalue_2 (`|CreateWidget` "/Game/UI/UI_MainMenu.UI_MainMenu_C" _returnvalue))
  (`UserWidget.AddToViewport` _returnvalue_2 0)
  (set `self.Menu` _returnvalue_2)
  (set `PlayerController.bShowMouseCursor` true _returnvalue))

(event `self.ReceiveTick`
  (params (DeltaSeconds :type "Float (single-precision)"))
  (bind _menu (`self.Menu`))
  (bind _menu_2 (`self.Menu`))
  (if (and (`CheckBox.IsChecked` (`/Game/UI/UI_MainMenu.P1_ReadyCheck` _menu)) (`CheckBox.IsChecked` (`/Game/UI/UI_MainMenu.P2_ReadyCheck` _menu)))
    (bind _astron_game_instance (cast `/Game/Blueprints/GameModes/TronGameInstance` (`GameplayStatics.GetGameInstance`)))
    (set `/Game/Blueprints/GameModes/TronGameInstance.P1_Power` (`ComboBoxString.GetSelectedOption` (`/Game/UI/UI_MainMenu.P1_PowerSelect` _menu_2)) _astron_game_instance)
    (set `/Game/Blueprints/GameModes/TronGameInstance.P2_Power` (`ComboBoxString.GetSelectedOption` (`/Game/UI/UI_MainMenu.P2_PowerSelect` _menu_2)) _astron_game_instance)
    (`GameplayStatics.OpenLevelBySoftObjectPtr` "/Game/Game.Game")))

(fn `UserConstructionScript`)